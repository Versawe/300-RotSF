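; Configurable elevator that moves a floor platform up and down inside a procedurally built pipe cage.
; Trigger and Toggle signals, each gated by a flag, run a timeline at height-scaled speed to move the Mover, while crank updates set its playback position.
; The construction script attaches listed items to the Mover, sets its starting height and builds the frame from instanced cylinders, with optional openings at top and bottom.
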(event EventBeginPlay
  (bind _percent (Timeline|MoveElevator SetNewTime)
    (:Update
      (Transformation|SetRelativeLocation (Variables|Default|GetMover) (Math|Vector|MakeVector 0.0 0.0 (* _percent (- (Variables|ElevatorSize|GetHow%20high?) (Variables|Default|GetCeiling%20Margin)) 1e+02)) false false))))

(event EventCrankWasUpdated
  (params (New%20Percent%20Value :type Float%20%28single-precision%29))
  (Components|Timeline|SetPlaybackPosition (Variables|Default|GetMoveElevator) (Math|Float|Clamp(Float) (select (Variables|ElevatorBehavior|GetIs%20Elevator%20Up) (- 1.0 New%20Percent%20Value) New%20Percent%20Value)) false true))

(event EventTrigger
  (if (Variables|ElevatorBehavior|GetAllow%20trigger%20signals)
    (Variables|ElevatorBehavior|SetIs%20Elevator%20Up (not (Variables|ElevatorBehavior|GetIs%20Elevator%20Up)))
    (Components|Timeline|SetPlayRate (Variables|Default|GetMoveElevator) (/ (Variables|ElevatorBehavior|GetSpeed) (Variables|ElevatorSize|GetHow%20high?)))
    (if (Variables|ElevatorBehavior|GetIs%20Elevator%20Up)
      (bind _percent (Timeline|MoveElevator Play)
        (:Update
          (Transformation|SetRelativeLocation (Variables|Default|GetMover) (Math|Vector|MakeVector 0.0 0.0 (* _percent (- (Variables|ElevatorSize|GetHow%20high?) (Variables|Default|GetCeiling%20Margin)) 1e+02)) false false)))
      (else
        (Timeline|MoveElevator Reverse)))))

(event EventToggle
  (params (IsNowOn :type Boolean))
  (if (Variables|ElevatorBehavior|GetAllow%20toggle%20signals)
    (Variables|ElevatorBehavior|SetIs%20Elevator%20Up IsNowOn)
    (Components|Timeline|SetPlayRate (Variables|Default|GetMoveElevator) (/ (Variables|ElevatorBehavior|GetSpeed) (Variables|ElevatorSize|GetHow%20high?)))
    (if (Variables|ElevatorBehavior|GetIs%20Elevator%20Up)
      (bind _percent (Timeline|MoveElevator Play)
        (:Update
          (Transformation|SetRelativeLocation (Variables|Default|GetMover) (Math|Vector|MakeVector 0.0 0.0 (* _percent (- (Variables|ElevatorSize|GetHow%20high?) (Variables|Default|GetCeiling%20Margin)) 1e+02)) false false)))
      (else
        (Timeline|MoveElevator Reverse)))))

(fn ConstructionScript
  (bind _how_high_ (Variables|ElevatorSize|GetHow%20high?))
  (bind _returnvalue (Math|Float|Truncate _how_high_))
  (bind _returnvalue_2 (- _returnvalue 1))
  (Utilities|FlowControl|Sequence
    (:then_0
      ;[1 1 1] Weld items to floor
      (for _array_element (Variables|ElevatorBehavior|GetWeld%20to%20floor)
        (Transformation|AttachComponentToComponent _array_element (Variables|Default|GetMover) "None" "KeepWorld" "KeepWorld" "KeepWorld" true)))
    (:then_1
      ;[1 1 1] Position floor and mover
      (Transformation|SetRelativeTransform (Variables|Default|GetMover) (Math|Transform|MakeTransform (Math|Vector|MakeVector 0.0 0.0 (select (Variables|ElevatorBehavior|GetIs%20Elevator%20Up) (* (- (Variables|ElevatorSize|GetHow%20high?) (Variables|Default|GetCeiling%20Margin)) 1e+02) 0.0)) "0, 0, 0" "1,1,1") false true)
      (Transformation|SetRelativeTransform (Variables|Default|GetMesh%20Floor) (Math|Transform|MakeTransform (Math|Vector|MakeVector 0.0 0.0 (Variables|Default|GetFloor%20Margin)) "0, 0, 0" (Math|Vector|MakeVector (Variables|ElevatorSize|GetWidth) (Variables|ElevatorSize|GetDepth) 0.05)) false true))
    (:then_2
      ;[1 1 1] Construct frame
      (CallFunction|MakeVerticalPipe false false 1e+01)
      (CallFunction|MakeVerticalPipe true false 1e+01)
      (CallFunction|MakeVerticalPipe false true 1e+01)
      (CallFunction|MakeVerticalPipe true true 1e+01)
      (bind _index (Utilities|FlowControl|ForLoopwithBreak 0 _returnvalue_2)
        (:LoopBody
          (if (< _index 2)
            (CallFunction|MakeHorizontalPipes (+ (* _index 1e+02) 5.0) 1e+01 (Variables|ElevatorDoors|GetAt%20bottom,%20open%20BACK) (Variables|ElevatorDoors|GetAt%20bottom,%20open%20FRONT) (Variables|ElevatorDoors|GetAt%20bottom,%20open%20LEFT) (Variables|ElevatorDoors|GetAt%20bottom,%20open%20RIGHT))
            (elif (>= _index _returnvalue_2)
              (CallFunction|MakeHorizontalPipes (+ (* _index 1e+02) 5.0) 1e+01 (Variables|ElevatorDoors|GetAt%20top,%20open%20BACK) (Variables|ElevatorDoors|GetAt%20top,%20open%20FRONT) (Variables|ElevatorDoors|GetAt%20top,%20open%20LEFT) (Variables|ElevatorDoors|GetAt%20top,%20open%20RIGHT))
              (else
                (CallFunction|MakeHorizontalPipes (+ (* _index 1e+02) 5.0) 1e+01 false false false false)))))
        (:Completed
          (CallFunction|MakeHorizontalPipes (+ (* (Variables|ElevatorSize|GetHow%20high?) 1e+02) 1e+01) 1e+01 false false false false))))))

(fn MakeVerticalPipe
  (params (Flip%20X :type Boolean) (Flip%20Y :type Boolean) (Offset :type Float%20%28single-precision%29))
  (Components|InstancedStaticMesh|AddInstance (Variables|Default|GetCylinders) (Math|Transform|MakeTransform (Math|Vector|MakeVector (* (+ (* (Variables|ElevatorSize|GetWidth) 5e+01) Offset) (select Flip%20X -1.0 1.0)) (* (+ (* (Variables|ElevatorSize|GetDepth) 5e+01) Offset) (select Flip%20Y -1.0 1.0)) (* (Variables|ElevatorSize|GetHow%20high?) 5e+01)) "0, 0, 0" (Math|Vector|MakeVector 0.1 0.1 (+ (Variables|ElevatorSize|GetHow%20high?) 0.5)))))

(fn MakeHorizontalPipes
  (params (Z%20Offset :type Float%20%28single-precision%29) (Lateral%20Offset :type Float%20%28single-precision%29) (Omit%20Back :type Boolean) (Omit%20Front :type Boolean) (Omit%20Left :type Boolean) (Omit%20Right :type Boolean))
  (bind _depth (Variables|ElevatorSize|GetDepth))
  (bind _width (Variables|ElevatorSize|GetWidth))
  (bind _returnvalue (/ Lateral%20Offset 2.0))
  (bind _returnvalue_2 (/ Lateral%20Offset 2.0))
  (bind _returnvalue_3 (* _width 5e+01))
  (bind _returnvalue_4 (* _depth 5e+01))
  (bind _returnvalue_5 (+ _returnvalue_3 Lateral%20Offset))
  (bind _returnvalue_6 (+ _returnvalue_4 Lateral%20Offset))
  (bind _returnvalue_7 (+ _returnvalue_5 _returnvalue_2))
  (bind _returnvalue_8 (+ _returnvalue_6 _returnvalue))
  (Utilities|FlowControl|Sequence
    (:then_0
      (if (not Omit%20Back)
        ;[1 1 1] Back
        (Components|InstancedStaticMesh|AddInstance (Variables|Default|GetCylinders) (Math|Transform|MakeTransform (Math|Vector|MakeVector 0.0 _returnvalue_8 Z%20Offset) "90.000000, 0,0.000000" (Math|Vector|MakeVector 0.07 0.07 (+ (Variables|ElevatorSize|GetWidth) (* Lateral%20Offset 0.04)))))))
    (:then_1
      (if (not Omit%20Front)
        ;[1 1 1] Front
        (Components|InstancedStaticMesh|AddInstance (Variables|Default|GetCylinders) (Math|Transform|MakeTransform (Math|Vector|MakeVector 0.0 (* _returnvalue_8 -1.0) Z%20Offset) "90.000000, 0,0.000000" (Math|Vector|MakeVector 0.07 0.07 (+ (Variables|ElevatorSize|GetWidth) (* Lateral%20Offset 0.04)))))))
    (:then_2
      (if (not Omit%20Left)
        ;[1 1 1] Left
        (Components|InstancedStaticMesh|AddInstance (Variables|Default|GetCylinders) (Math|Transform|MakeTransform (Math|Vector|MakeVector _returnvalue_7 0.0 (+ _returnvalue_2 Z%20Offset)) "0.000000, 0,90.000000" (Math|Vector|MakeVector 0.07 0.07 (+ (Variables|ElevatorSize|GetDepth) (* Lateral%20Offset 0.04)))))))
    (:then_3
      (if (not Omit%20Right)
        ;[1 1 1] Right
        (Components|InstancedStaticMesh|AddInstance (Variables|Default|GetCylinders) (Math|Transform|MakeTransform (Math|Vector|MakeVector (* _returnvalue_7 -1.0) 0.0 (+ (/ Lateral%20Offset 2.0) Z%20Offset)) "0.000000, 0,90.000000" (Math|Vector|MakeVector 0.07 0.07 (+ (Variables|ElevatorSize|GetDepth) (* Lateral%20Offset 0.04)))))))))

(fn GetFloorPositionatTop)