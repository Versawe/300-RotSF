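; Interactable push button actor that the player can press while standing inside its trigger box.
; Box overlap with the PlayerCharacter enables or disables input on the button, so Interact only works in range.
; Pressing plays a click sound, fires the ButtonWasPushed dispatcher for other objects, and runs a timeline that slides the button mesh along its local X axis.
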(event OnComponentBeginOverlap(Box)
  (params (OverlappedComponent :type Primitive%20Component%20Object%20Reference) (OtherActor :type Actor%20Object%20Reference) (OtherComp :type Primitive%20Component%20Object%20Reference) (OtherBodyIndex :type Integer) (bFromSweep :type Boolean) (SweepResult :type Hit%20Result%20Structure%20%28by%20ref%29))
  ;[0.2578 1 0.1939] Specify Player Overlap with Button
  (Utilities|Casting|CastToPlayerCharacter OtherActor)
  (Input|EnableInput (Game|GetPlayerController 0)))

(event OnComponentEndOverlap(Box)
  (params (OverlappedComponent :type Primitive%20Component%20Object%20Reference) (OtherActor :type Actor%20Object%20Reference) (OtherComp :type Primitive%20Component%20Object%20Reference) (OtherBodyIndex :type Integer))
  ;[0.2578 1 0.1939] Specify Player Overlap with Button
  (Utilities|Casting|CastToPlayerCharacter OtherActor)
  (Input|DisableInput (Game|GetPlayerController 0)))

(event EventBeginPlay)

(event Input|ActionEvents|InputActionInteract
  (params (Key :type Key%20Structure :default "None"))
  ;[1 0.125 0.125] Button Animation
  (:Pressed
    (Audio|PlaySoundatLocation "/Engine/VREditor/Sounds/UI/Click_on_Button_Cue.Click_on_Button_Cue" (Transformation|GetActorLocation) "0, 0, 0" 1.0 1.0 0.0 0 0 0)
    (Default|CallTheButtonWasPushed)
    (bind _relative_x (Timeline|button%20pressed PlayFromStart)
      (:Update
        (Transformation|SetRelativeLocation (Variables|Default|GetMoveable%20Button) (Math|Vector|MakeVector _relative_x 0.0 0.0) false false)))))

(fn ConstructionScript)